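; Enemy NPC AI that wanders to random reachable points until Pawn Sensing spots a pawn, then triggers that pawn's detection message.
; A retriggerable delay clears the message when sightings stop.
; It chases seen pawns only while Startchace's flag is set; StopChace halts it and resumes wandering.
; Capsule contact with BP_FirstPersonCharacter disables input, plays a punch via Tick, shows the Wyakalandin widget, then plays the Ending sequence.
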(event OnSeePawn(PawnSensing)
  (params (Pawn :type Pawn%20Object%20Reference))
  (Variables|Default|SetDetedtedplayer Pawn)
  (Utilities|FlowControl|Sequence
    (:then_0
      (Utilities|FlowControl|Sequence
        (:then_0
          (Utilities|FlowControl|DoOnce false :!label _label
            (:Completed
              (Class|BpDetection|StartDetection(Message) (Variables|Default|GetDetedtedplayer) self)
              (Development|PrintText "gördü")
              (bind _output_get (Variables|Default|Setrast true))
              (if (not _output_get)
                (AI|AIMoveTo self (.RandomLocation (AI|Navigation|GetRandomReachablePointinRadius (Transformation|GetWorldLocation (Variables|Character|GetMesh)) 2e+03 0 0)) 0 5.0 false
                  (:then
                    (Utilities|FlowControl|Delay 5.0)
                    (CallFunction|CustomEvent)))))))
        (:then_1
          (if (Variables|Default|GetShould%20Case?)
            (CallFunction|ChasePlayer (Variables|Default|GetDetedtedplayer))))))
    (:then_1
      (Variables|Default|Setrast true)
      (Utilities|FlowControl|RetriggerableDelay 1.5)
      (Class|BpDetection|Stopdetection(Message) (Variables|Default|GetDetedtedplayer))
      (goto _label Reset))))

(event OnComponentHit(CapsuleComponent)
  (params (HitComponent :type Primitive%20Component%20Object%20Reference) (OtherActor :type Actor%20Object%20Reference) (OtherComp :type Primitive%20Component%20Object%20Reference) (NormalImpulse :type Vector :default "0, 0, 0") (Hit :type Hit%20Result%20Structure%20%28by%20ref%29))
  (bind _asbp_first_person_character (Utilities|Casting|CastToBP_FirstPersonCharacter OtherActor))
  (Collision|SetCollisionEnabled (Variables|Collision|GetCapsuleComponent) "NoCollision")
  (bind _output_get (Variables|Default|Setdoku true))
  (Input|DisableInput _asbp_first_person_character 0)
  (Utilities|FlowControl|Delay 1.0)
  (bind _returnvalue (UserInterface|CreateWidget "/Game/npc/wyakalandin.wyakalandin_C"))
  (UserInterface|Viewport|AddtoViewport _returnvalue 0)
  (Utilities|FlowControl|Delay 1.5)
  (Viewport|RemoveAllWidgets)
  (bind _returnvalue_2 (Sequencer|Player|CreateLevelSequencePlayer "/Game/sequence/Ending.Ending"))
  (Sequencer|Player|Play _returnvalue_2 :!class /Script/MovieScene.MovieSceneSequencePlayer))

(event Custom|Chase%20Player
  (params (TargetActor :type Actor%20Object%20Reference))
  (AI|AIMoveTo self "0, 0, 0" TargetActor 5.0 false))

(event Custom|CustomEvent
  (Utilities|FlowControl|Delay 3.0)
  (if (not (stale OnSeePawn(PawnSensing) _output_get))
    (AI|AIMoveTo self (.RandomLocation (AI|Navigation|GetRandomReachablePointinRadius (Transformation|GetWorldLocation (Variables|Character|GetMesh)) 2e+03 0 0)) 0 5.0 false
      (:then
        (Utilities|FlowControl|Delay 5.0)
        (CallFunction|CustomEvent)))))

(event EventBeginPlay
  (if (not (stale OnSeePawn(PawnSensing) _output_get))
    (CallFunction|CustomEvent)))

(event Collision|EventActorBeginOverlap
  (params (OtherActor :type Actor%20Object%20Reference)))

(event EventTick
  (params (DeltaSeconds :type Float%20%28single-precision%29))
  (if (stale OnComponentHit(CapsuleComponent) _output_get)
    (Utilities|FlowControl|DoOnce false
      (:Completed
        (Components|Animation|PlayAnimation (Variables|Character|GetMesh) "/Game/npc/Mutant_Punch.Mutant_Punch" false)))))

(event EventStopChace
  (bind _self self)
  (Variables|Default|SetShould%20Case? false)
  (AI|AIMoveTo _self "0, 0, 0" _self 5.0 false
    (:then
      (Variables|Default|Setrast false)
      (CallFunction|CustomEvent))))

(event EventStartchace
  (Variables|Default|SetShould%20Case? true))

(fn ConstructionScript)