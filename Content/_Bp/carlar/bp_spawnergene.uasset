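; Timed spawner actor that periodically swaps its child actor among three configurable classes.
; Tick feeds a Delay of random 10 to 30 second length, making a repeating timer that picks a class at random and sets it on the ChildActor component.
; BeginPlay starts a two-minute countdown, after which the spawner destroys itself.
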(event EventBeginPlay
  (Utilities|FlowControl|Delay 1.2e+02)
  (Actor|DestroyActor))

(event Collision|EventActorBeginOverlap
  (params (OtherActor :type Actor%20Object%20Reference)))

(event EventTick
  (params (DeltaSeconds :type Float%20%28single-precision%29))
  (Utilities|FlowControl|Delay (Math|Random|RandomFloatinRange 1e+01 3e+01))
  (bind _output_get (Variables|Default|SetNewVar_seciliii (Utilities|Select :Index (Math|Random|RandomIntegerinRange 0 2) :Option%200 (Variables|Default|GetNewVar) :Option%201 (Variables|Default|GetNewVar_0) :Option%202 (Variables|Default|GetNewVar_1))))
  (ChildActorComponent|SetChildActorClass (Variables|Default|GetChildActor) _output_get))

(fn ConstructionScript)