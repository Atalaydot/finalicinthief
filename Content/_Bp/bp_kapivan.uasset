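; Van door Blueprint that swings a Cube mesh open and closed when the kapitik event is called.
; A FlipFlop alternately plays and reverses a timeline that lerps the Cube's relative yaw between closed and open, with a car lock/unlock sound on each toggle.
; On BeginPlay the Cube is hidden, then shown again after a short delay.
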(event Custom|kapitik
  (Utilities|FlowControl|FlipFlop
    (:A
      (Audio|PlaySound2D "/Game/effect/car-lock-and-unlock-47502.car-lock-and-unlock-47502" 1.0 1.0 0.0 0 0)
      (bind _newtrack_0 (Timeline|Zaman%20Çizelgesi Play)
        (:Update
          (Transformation|SetRelativeRotation (Variables|Default|GetCube) (Math|Rotator|MakeRotator 0.0 0.0 (Math|Float|Lerp 0.0 -5e+01 _newtrack_0)) false false))))
    (:B
      (Audio|PlaySound2D "/Game/effect/car-lock-and-unlock-47502.car-lock-and-unlock-47502" 1.0 1.0 0.0 0 0)
      (Timeline|Zaman%20Çizelgesi Reverse))))

(event EventBeginPlay
  (Rendering|SetVisibility (Variables|Default|GetCube) false false)
  (Utilities|FlowControl|Delay 5.0)
  (Rendering|SetVisibility (Variables|Default|GetCube) true false))

(event Collision|EventActorBeginOverlap
  (params (OtherActor :type Actor%20Object%20Reference)))

(fn ConstructionScript)