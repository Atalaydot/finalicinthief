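; Door actor that swings open and closed, with a proximity prompt widget.
; The tiklamakapi event alternates via FlipFlop between playing and reversing a timeline that lerps the Cube's yaw between 0 and -60 degrees, with a 2D sound each time.
; A Box overlap shows the widget only until the door is first used, tracked by the Okey flag, and hides it on exit.
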(event OnComponentBeginOverlap(Box)
  (params (OverlappedComponent :type Primitive%20Component%20Object%20Reference) (OtherActor :type Actor%20Object%20Reference) (OtherComp :type Primitive%20Component%20Object%20Reference) (OtherBodyIndex :type Integer) (bFromSweep :type Boolean) (SweepResult :type Hit%20Result%20Structure%20%28by%20ref%29))
  (if (not (Variables|Default|Getokey))
    (Rendering|SetVisibility (Variables|Default|GetWidget) true false)))

(event OnComponentEndOverlap(Box)
  (params (OverlappedComponent :type Primitive%20Component%20Object%20Reference) (OtherActor :type Actor%20Object%20Reference) (OtherComp :type Primitive%20Component%20Object%20Reference) (OtherBodyIndex :type Integer))
  (Rendering|SetVisibility (Variables|Default|GetWidget) false false))

(event Custom|tiklama%20kapi
  (Variables|Default|Setokey true)
  (Utilities|FlowControl|FlipFlop
    (:A
      (Audio|PlaySound2D "/Game/effect/opendoor.opendoor" 1.0 1.0 0.0 0 0)
      (bind _doorrotation (Timeline|Doortimeline Play)
        (:Update
          (Transformation|SetRelativeRotation (Variables|Default|GetCube) (Math|Rotator|MakeRotator 0.0 0.0 (Math|Float|Lerp 0.0 -6e+01 _doorrotation)) false false))))
    (:B
      (Audio|PlaySound2D "/Game/effect/opendoor.opendoor" 1.0 1.0 0.0 0 0)
      (Timeline|Doortimeline Reverse))))

(event EventBeginPlay)

(event Collision|EventActorBeginOverlap
  (params (OtherActor :type Actor%20Object%20Reference)))

(event EventTick
  (params (DeltaSeconds :type Float%20%28single-precision%29)))

(fn ConstructionScript)